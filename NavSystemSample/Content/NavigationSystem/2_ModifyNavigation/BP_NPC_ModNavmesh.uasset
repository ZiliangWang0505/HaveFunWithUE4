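; BP_NPC_ModNavmesh is an NPC that endlessly roams between randomly chosen actors from its TargetList in a navmesh modification setup.
; MoveNPC starts on BeginPlay, picks a reachable point near a valid target and calls AI MoveTo, optionally drawing a debug sphere there.
; It calls itself again after a pause on success or a brief retry delay on failure, but an invalid target ends the loop.
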(event `self.ReceiveBeginPlay`
  (`self.MoveNPC`))

(event `MoveNPC`
  (bind _targetlist (`self.TargetList`))
  (bind _output_get (set `self.CurrentTarget` (`|GetArrayItem` _targetlist (`KismetMathLibrary.RandomIntegerInRange` 0 (`KismetArrayLibrary.Array_LastIndex` _targetlist)))))
  (`/Engine/EditorBlueprintResources/StandardMacros.IsValid` _output_get
    (:`Is Valid`
      (bind _output_get_2 (set `self.RandomLocation` (`NavigationSystemV1.K2_GetRandomReachablePointInRadius` (`self.K2_GetActorLocation` (`self.CurrentTarget`)) 100.0 null null)))
      (`|AIMoveTo` self _output_get_2 null 50.0
        (:`then`
          (if (`self.ShowTarget`)
            (`KismetSystemLibrary.DrawDebugSphere` (`self.RandomLocation`) 100.0 12 (`self.SphereColor`) 5.0 10.0)))
        (:`OnSuccess`
          (`KismetSystemLibrary.Delay` 4.0)
          (`self.MoveNPC`))
        (:`OnFail`
          (`KismetSystemLibrary.Delay` 0.1)
          (`self.MoveNPC`))))))

(fn `UserConstructionScript`)