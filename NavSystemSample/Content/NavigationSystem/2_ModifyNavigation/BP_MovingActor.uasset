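; BP_MovingActor is an actor in the navigation-modification folder whose mesh shuttles back and forth along its relative X axis.
; BeginPlay starts the TM_MoveObject timeline, whose alpha interpolates the mesh's X location between zero and Distance.
; When the timeline finishes, a short delay precedes a flip of the Forward flag, which selects reversing or replaying the timeline for an endless loop.
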(event `self.ReceiveBeginPlay`
  (`self.MoveForward`))

(event `MoveForward`
  (bind (_direction _alpha) (`Timeline|TM_MoveObject` :!label _label)
    (:`Update`
      (`SceneComponent.K2_SetRelativeLocation` (`self.Mesh`) (`KismetMathLibrary.MakeVector` (`KismetMathLibrary.Lerp` 0.0 (`self.Distance`) _alpha)) false false))
    (:`Finished`
      (`KismetSystemLibrary.Delay` 1.0)
      (if (`self.Forward`)
        (set `self.Forward` false)
        (`self.MoveBackwards`)
        (else
          (set `self.Forward` true)
          (`self.MoveForward`))))))

(event `MoveBackwards`
  (goto _label :!via `Reverse`))

(fn `UserConstructionScript`)