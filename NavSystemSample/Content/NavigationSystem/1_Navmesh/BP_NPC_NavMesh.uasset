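; NPC Blueprint for a navmesh setup that wanders continuously between random reachable points.
; On BeginPlay it picks a reachable point within a radius of its current location and issues an AI MoveTo to it.
; The move event calls itself again after a pause on success, or almost immediately on failure.
; An optional debug sphere marks each chosen destination.
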(event `self.ReceiveBeginPlay`
  (`self.MoveNPC`))

(event `MoveNPC`
  (bind _output_get (set `self.RandomLocation` (`NavigationSystemV1.K2_GetRandomReachablePointInRadius` (`self.K2_GetActorLocation`) 3000.0 null null)))
  (`|AIMoveTo` self _output_get null
    (:`then`
      (if (`self.ShowTarget`)
        (`KismetSystemLibrary.DrawDebugSphere` (`self.RandomLocation`) 100.0 12 (`self.SphereColor`) 5.0 10.0)))
    (:`OnSuccess`
      (`KismetSystemLibrary.Delay` 4.0)
      (`self.MoveNPC`))
    (:`OnFail`
      (`KismetSystemLibrary.Delay` 0.1)
      (`self.MoveNPC`))))

(fn `UserConstructionScript`)