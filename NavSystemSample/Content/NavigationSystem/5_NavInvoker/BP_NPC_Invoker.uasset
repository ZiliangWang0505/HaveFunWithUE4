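; BP_NPC_Invoker is a wandering NPC, filed under the navigation invoker section of a NavigationSystem folder.
; On BeginPlay it picks a random reachable point within a radius of its current location and walks there with AI MoveTo.
; MoveNPC then calls itself again, after a pause on success or a much shorter retry delay on failure, so the roaming loops indefinitely.
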(event `self.ReceiveBeginPlay`
  (`self.MoveNPC`))

(event `MoveNPC`
  (set `self.TargetLocation` (`NavigationSystemV1.K2_GetRandomReachablePointInRadius` (`self.K2_GetActorLocation`) 2500.0 null null))
  (`|AIMoveTo` self (`self.TargetLocation`) null
    (:`OnSuccess`
      (`KismetSystemLibrary.Delay` 5.0)
      (`self.MoveNPC`))
    (:`OnFail`
      (`KismetSystemLibrary.Delay` 0.2)
      (`self.MoveNPC`))))

(fn `UserConstructionScript`)